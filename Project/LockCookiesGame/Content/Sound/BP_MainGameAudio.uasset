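; BP_MainGameAudio is the actor that plays the main game music, holding it back until the intro cinematic ends.
; On BeginPlay it stops its Audio component and binds to the game mode's FinishCinematic dispatcher, which starts playback from the beginning.
; Every tick it sets the music's pitch multiplier from the game mode's music rate.
; An OnBeat event plays a 2D Jump sound, with no caller shown here.
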(event Custom|OnBeat
  (Audio|PlaySound2D "/Game/Sound/Jump.Jump" 1.0 1.0 0.0 0 0))

(event Custom|FinishCinematic
  (Audio|Components|Audio|Play (Variables|Default|GetAudio) 0.0))

(event EventBeginPlay
  (Audio|Components|Audio|Stop (Variables|Default|GetAudio))
  (bind _asbp_main_game_mode (Utilities|Casting|CastToBP_MainGameMode (Game|GetGameMode)))
  (bind _output_get (Variables|Default|SetAs%20BP%20Main%20Game%20Mode _asbp_main_game_mode))
  (EventDispatchers|AssignFinishCinematicDispatch _output_get (delegate Custom|FinishCinematic)))

(event EventTick
  (params (DeltaSeconds :type Float%20%28single-precision%29))
  (bind _rate (Default|GetGameMusicRate (Variables|Default|GetAs%20BP%20Main%20Game%20Mode)))
  (Audio|Components|Audio|SetPitchMultiplier (Variables|Default|GetAudio) _rate))

(fn ConstructionScript)