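; BP_MainPlayerController is the player controller that drives movement and jumping for BP_MainCharacter.
; It caches the controlled character on BeginPlay and, while EnableMovement is set, pushes it along its forward vector every Tick.
; MoveX and MoveY axes add input along world Y and X respectively, independent of camera or character rotation.
; The Jump action re-casts the controlled pawn before calling Jump.
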(event EventBeginPlay
  (bind _asbp_main_character (Utilities|Casting|CastToBP_MainCharacter (Pawn|GetControlledPawn)))
  (Variables|Default|SetMainCharacter _asbp_main_character))

(event EventTick
  (params (DeltaSeconds :type Float%20%28single-precision%29))
  (bind _maincharacter (Variables|Default|GetMainCharacter))
  (if (Variables|Default|GetEnableMovement)
    (Pawn|Input|AddMovementInput _maincharacter (Transformation|GetActorForwardVector _maincharacter) 1.0 false)))

(event Input|ActionEvents|InputActionJump
  (params (Key :type Key%20Structure :default "None"))
  (:Pressed
    (bind _asbp_main_character (Utilities|Casting|CastToBP_MainCharacter (Pawn|GetControlledPawn)))
    (Character|Jump _asbp_main_character)))

(event Input|AxisEvents|InputAxisMoveX
  (params (AxisValue :type Float%20%28single-precision%29))
  (Pawn|Input|AddMovementInput (Variables|Default|GetMainCharacter) (Math|Vector|MakeVector 0.0 AxisValue 0.0) 1.0 false))

(event Input|AxisEvents|InputAxisMoveY
  (params (AxisValue :type Float%20%28single-precision%29))
  (Pawn|Input|AddMovementInput (Variables|Default|GetMainCharacter) (Math|Vector|MakeVector AxisValue 0.0 0.0) 1.0 false))

(fn ConstructionScript)