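; BP_FollowerActor is a follower character actor with a randomized look that can be switched on and off.
; Its construction script gives the mesh a dynamic MI_Boy_salsa material with a random whole-number "randomNum" parameter for per-instance variation.
; OnEnable and OnDisable toggle visibility, but both leave the capsule at QueryOnly collision because the disable check is inverted.
; A random BaseColor assignment is left unconnected.
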(event Custom|OnDisable
  (bind _output_get (Variables|Default|SetIsEnabled false))
  (Rendering|SetActorHiddenInGame (not _output_get))
  (Collision|SetCollisionEnabled (Variables|Default|GetCapsule) (select (not _output_get) "QueryOnly" "NoCollision")))

(event Custom|OnEnable
  (bind _output_get (Variables|Default|SetIsEnabled true))
  (Rendering|SetActorHiddenInGame (not _output_get))
  (Collision|SetCollisionEnabled (Variables|Default|GetCapsule) (select _output_get "QueryOnly" "NoCollision")))

(event EventBeginPlay)

(fn ConstructionScript
  (bind _returnvalue (Rendering|Material|CreateDynamicMaterialInstance (Variables|Default|GetMesh) 0 "/Game/Mesh/Boy_VAT/SalsaMovement/MI_Boy_salsa.MI_Boy_salsa" "None" :!class /Script/Engine.PrimitiveComponent))
  (bind _output_get (Variables|Default|SetMaterialInstance _returnvalue))
  (Rendering|Material|SetScalarParameterValue _output_get "randomNum" (Math|Conversions|ToFloat(Integer) (Math|Float|Round (Math|Random|RandomFloatinRange 0.0 31.0))) :!class /Script/Engine.MaterialInstanceDynamic))