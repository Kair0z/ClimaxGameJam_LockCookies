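; Player character that leads a chain of followers through a SnakeFollowComponent and ends the round through the main game mode on a frontal collision.
; Spawns initial followers at BeginPlay; each addition plays a random cheer and triggers a jump.
; Every tick, it scales walk speed by the game mode's rate and sprint bonus, and raises follower interpolation rate with the sprint bonus.
; Jump and landing events track airborne state.
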(event Custom|AddFollowers
  (params (Num :type Integer))
  (Default|AddFollowers (Variables|Default|GetSnakeFollowComponent) Num)
  (Audio|PlaySound2D (select (Math|Random|RandomBool) "/Game/Sound/YEAH2.YEAH2" "/Game/Sound/YEAH.YEAH") 0.6 1.0 0.0 0 0)
  (Character|Jump))

(event Custom|OnFrontalCollision
  (Default|OnEndOfRound (Variables|Default|GetAs%20BP%20Main%20Game%20Mode_0)))

(event Custom|SetMovementRate
  (params (Rate :type Float%20%28single-precision%29))
  (Variables|/Script/Engine.CharacterMovementComponent|SetMaxWalkSpeed (Variables|Character|GetCharacterMovement) (* (+ (Variables|Default|GetBaseWalkSpeed) (Variables|Default|GetSprintMultiplier)) Rate)))

(event EventBeginPlay
  (Variables|/Script/Engine.CharacterMovementComponent|SetMaxWalkSpeed (Variables|Character|GetCharacterMovement) (Variables|Default|GetBaseWalkSpeed))
  (bind _asbp_main_game_mode (Utilities|Casting|CastToBP_MainGameMode (Game|GetGameMode)))
  (Variables|Default|SetAs%20BP%20Main%20Game%20Mode _asbp_main_game_mode)
  (CallFunction|AddFollowers (Variables|Default|GetInitialSpawnAmountOfPlayers))
  (bind _asbp_main_game_mode_2 (Utilities|Casting|CastToBP_MainGameMode (Game|GetGameMode)))
  (Variables|Default|SetAs%20BP%20Main%20Game%20Mode_0 _asbp_main_game_mode_2))

(event EventTick
  (params (DeltaSeconds :type Float%20%28single-precision%29))
  (bind _snakefollowcomponent (Variables|Default|GetSnakeFollowComponent))
  (bind _rate (Default|GetGameRate (Variables|Default|GetAs%20BP%20Main%20Game%20Mode)))
  (CallFunction|SetMovementRate _rate)
  (Variables|/Game/Blueprints/Player/BPC_SnakeFollowComponent.BPC_SnakeFollowComponent_C|SetInterpolationRateHorVert_Current _snakefollowcomponent (+ (Variables|/Game/Blueprints/Player/BPC_SnakeFollowComponent.BPC_SnakeFollowComponent_C|GetInterpolationRateHorVert_Base _snakefollowcomponent) (* (Math|Vector2D|MakeVector2D 0.1 0.1) (Variables|Default|GetSprintMultiplier)))))

(event EventOnJumped
  (Variables|Default|SetIsInAir true)
  (Audio|PlaySound2D "/Game/Sound/Jump.Jump" 1.0 1.0 0.0 0 0))

(event EventOnLanded
  (params (Hit :type Hit%20Result%20Structure%20%28by%20ref%29))
  (Variables|Default|SetIsInAir false))

(fn ConstructionScript)

(fn GetCurrentNumFollowers
  (return (Variables|/Game/Blueprints/Player/BPC_SnakeFollowComponent.BPC_SnakeFollowComponent_C|GetNumFollowers (Variables|Default|GetSnakeFollowComponent))))