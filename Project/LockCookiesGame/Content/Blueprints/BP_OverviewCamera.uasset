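; BP_OverviewCamera is an actor that smoothly follows the main character, named as the game's overview camera.
; On BeginPlay it casts the game mode to BP_MainGameMode and caches it, which provides the main character reference.
; Each Tick it moves itself toward that character's location with VInterpTo at InterpSpeed, without sweeping, and leaves rotation untouched.
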(event EventBeginPlay
  (bind _asbp_main_game_mode (Utilities|Casting|CastToBP_MainGameMode (Game|GetGameMode)))
  (Variables|Default|SetAs%20BP%20Main%20Game%20Mode _asbp_main_game_mode))

(event EventTick
  (params (DeltaSeconds :type Float%20%28single-precision%29))
  (Transformation|SetActorLocation (Math|Interpolation|VInterpTo (Transformation|GetActorLocation) (Transformation|GetActorLocation (Variables|/Game/Blueprints/BP_MainGameMode.BP_MainGameMode_C|GetAs%20BP%20Main%20Character (Variables|Default|GetAs%20BP%20Main%20Game%20Mode))) DeltaSeconds (Variables|Default|GetInterp%20Speed)) false false))

(fn ConstructionScript)