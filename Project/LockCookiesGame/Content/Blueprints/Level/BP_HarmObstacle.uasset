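; BP_HarmObstacle is a level obstacle that harms the main character and its snake of followers on overlap.
; It caches the main game mode on BeginPlay to reach the main character.
; Overlap by the main character triggers its frontal collision handler.
; Overlap by a follower cuts off the character's SnakeFollowComponent chain at that follower's index.
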(event Collision|EventActorBeginOverlap
  (params (OtherActor :type Actor%20Object%20Reference))
  (bind _as_bp_main_game_mode (Variables|Default|GetAs%20BP%20Main%20Game%20Mode))
  (bind _as_bp_main_character (Variables|/Game/Blueprints/BP_MainGameMode.BP_MainGameMode_C|GetAs%20BP%20Main%20Character _as_bp_main_game_mode))
  (Utilities|FlowControl|Sequence
    (:then_0
      (if (== _as_bp_main_character OtherActor)
        (Default|OnFrontalCollision _as_bp_main_character)))
    (:then_1
      (bind _asbp_follower_actor (Utilities|Casting|CastToBP_FollowerActor OtherActor))
      (Default|CutoffatIndex (Variables|/Game/Blueprints/Player/BP_MainCharacter.BP_MainCharacter_C|GetSnakeFollowComponent _as_bp_main_character) (Variables|/Game/Blueprints/Player/BP_FollowerActor.BP_FollowerActor_C|GetFollowerIndex _asbp_follower_actor)))))

(event EventBeginPlay
  (bind _asbp_main_game_mode (Utilities|Casting|CastToBP_MainGameMode (Game|GetGameMode)))
  (Variables|Default|SetAs%20BP%20Main%20Game%20Mode _asbp_main_game_mode))

(fn ConstructionScript)