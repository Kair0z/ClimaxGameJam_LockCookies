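; BP_Chest is a level chest that opens when the main character overlaps it with enough followers.
; On BeginPlay it shows the required count in a gate widget, hides the treasure and caches the main game mode.
; A qualifying overlap opens it once by rotating StaticMesh1 and revealing the treasure.
; A chest flagged as master also calls WinRound on the game mode.
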(event EventBeginPlay
  (bind _returnvalue (UserInterface|CreateWidget "/Game/Blueprints/UI/BPW_GateWidget.BPW_GateWidget_C" (Game|GetPlayerController 0)))
  (UserInterface|SetWidget (Variables|Default|GetWidget) _returnvalue)
  (Rendering|Components|TextRender|SetText (Variables|/Game/Blueprints/UI/BPW_GateWidget.BPW_GateWidget_C|GetNumPlayersReq _returnvalue) (Utilities|Text|ToText(Integer) (Variables|Default|GetNumber)))
  (bind _asbp_main_game_mode (Utilities|Casting|CastToBP_MainGameMode (Game|GetGameMode)))
  (Variables|Default|SetAs%20BP%20Main%20Game%20Mode _asbp_main_game_mode)
  (Rendering|SetVisibility (Variables|Default|GetTreasure) false false))

(event Collision|EventActorBeginOverlap
  (params (OtherActor :type Actor%20Object%20Reference))
  (bind _asbp_main_character (Utilities|Casting|CastToBP_MainCharacter OtherActor))
  (bind _newparam (Default|GetCurrentNumFollowers _asbp_main_character))
  (if (>= _newparam (Variables|Default|GetNumber))
    (Utilities|FlowControl|DoOnce false
      (:Completed
        (Transformation|AddLocalRotation (Variables|Default|GetStaticMesh1) "0, 0,-50.000000" false false)
        (Rendering|SetVisibility (Variables|Default|GetTreasure) true false)
        (if (Variables|Default|GetIsMasterChest)
          ;[1 1 1] WIN
          (Default|WinRound (Variables|Default|GetAs%20BP%20Main%20Game%20Mode)))))))

(fn ConstructionScript)