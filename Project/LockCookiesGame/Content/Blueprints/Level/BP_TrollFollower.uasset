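; BP_TrollFollower is a level pickup that changes the main character's follower count by a random amount on overlap, then destroys itself.
; The amount is a rounded random float between MinMax.X and MinMax.Y, passed to BP_MainCharacter's AddFollowers.
; The construction script tints the mesh green through a dynamic instance of MI_ChibiSalsa.
; A looping respawn timer starts on BeginPlay, but its Respawn event is empty.
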(event Custom|Respawn)

(event EventBeginPlay
  (Utilities|Time|SetTimerbyEvent (delegate Custom|Respawn) (Variables|Default|GetTimeBetweenRespawn) true))

(event Collision|EventActorBeginOverlap
  (params (OtherActor :type Actor%20Object%20Reference))
  (bind _minmax (Variables|Default|GetMinMax))
  (bind (_x _y) (Math|Vector2D|BreakVector2D _minmax))
  (bind _asbp_main_character (Utilities|Casting|CastToBP_MainCharacter OtherActor))
  (Default|AddFollowers _asbp_main_character (Math|Float|Round (Math|Random|RandomFloatinRange _x _y)))
  (Actor|DestroyActor))

(fn ConstructionScript
  (bind _returnvalue (Rendering|Material|CreateDynamicMaterialInstance (Variables|Default|GetStaticMesh) 0 "/Game/Materials/MI_ChibiSalsa.MI_ChibiSalsa" "None" :!class /Script/Engine.PrimitiveComponent))
  (bind _output_get (Variables|Default|SetMaterial%20Instance _returnvalue))
  (Rendering|Material|SetMaterial (Variables|Default|GetStaticMesh) 0 _output_get)
  (Rendering|Material|SetVectorParameterValue (Variables|Default|GetMaterial%20Instance) "BaseColor" "(R=0.000000,G=0.348958,B=0.027052,A=1.000000)" :!class /Script/Engine.MaterialInstanceDynamic))