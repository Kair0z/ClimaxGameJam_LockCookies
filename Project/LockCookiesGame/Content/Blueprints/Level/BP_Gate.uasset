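; BP_Gate is a level gate that lets the player into the arena once they have gathered enough followers.
; On BeginPlay it fills a widget component with a BPW_GateWidget showing the required count and caches the main game mode.
; When a BP_MainCharacter overlaps the trigger box with enough followers, the gate destroys itself and calls PlayerEnterArena on the game mode.
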(event OnComponentBeginOverlap(TriggerBox)
  (params (OverlappedComponent :type Primitive%20Component%20Object%20Reference) (OtherActor :type Actor%20Object%20Reference) (OtherComp :type Primitive%20Component%20Object%20Reference) (OtherBodyIndex :type Integer) (bFromSweep :type Boolean) (SweepResult :type Hit%20Result%20Structure%20%28by%20ref%29))
  (bind _asbp_main_character (Utilities|Casting|CastToBP_MainCharacter OtherActor))
  (bind _newparam (Default|GetCurrentNumFollowers _asbp_main_character))
  (if (>= _newparam (Variables|Default|GetNumPlayersRequired))
    (Actor|DestroyActor)
    (Default|PlayerEnterArena (Variables|Default|GetAs%20BP%20Main%20Game%20Mode))))

(event EventBeginPlay
  (bind _returnvalue (UserInterface|CreateWidget "/Game/Blueprints/UI/BPW_GateWidget.BPW_GateWidget_C" (Game|GetPlayerController 0)))
  (UserInterface|SetWidget (Variables|Default|GetWidget) _returnvalue)
  (Rendering|Components|TextRender|SetText (Variables|/Game/Blueprints/UI/BPW_GateWidget.BPW_GateWidget_C|GetNumPlayersReq _returnvalue) (Utilities|Text|ToText(Integer) (Variables|Default|GetNumPlayersRequired)))
  (bind _asbp_main_game_mode (Utilities|Casting|CastToBP_MainGameMode (Game|GetGameMode)))
  (Variables|Default|SetAs%20BP%20Main%20Game%20Mode _asbp_main_game_mode))

(fn ConstructionScript)