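; BP_Follower is a collectible follower that the player picks up by touching it.
; When BP_MainCharacter overlaps it, it calls AddFollowers on the character to add one, then destroys itself.
; The construction script gives its skeletal mesh a dynamic instance of M_Base tinted green through the BaseColor parameter.
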(event EventBeginPlay)

(event Collision|EventActorBeginOverlap
  (params (OtherActor :type Actor%20Object%20Reference))
  (bind _asbp_main_character (Utilities|Casting|CastToBP_MainCharacter OtherActor))
  (Default|AddFollowers _asbp_main_character 1)
  (Actor|DestroyActor))

(event EventTick
  (params (DeltaSeconds :type Float%20%28single-precision%29)))

(fn ConstructionScript
  (bind _returnvalue (Rendering|Material|CreateDynamicMaterialInstance (Variables|Default|GetSkeletalMesh) 0 "/Game/Materials/M_Base.M_Base" "None" :!class /Script/Engine.PrimitiveComponent))
  (bind _output_get (Variables|Default|SetMaterial%20Instance _returnvalue))
  (Rendering|Material|SetMaterial (Variables|Default|GetSkeletalMesh) 0 _output_get)
  (Rendering|Material|SetVectorParameterValue (Variables|Default|GetMaterial%20Instance) "BaseColor" "(R=0.000000,G=0.348958,B=0.027052,A=1.000000)" :!class /Script/Engine.MaterialInstanceDynamic))